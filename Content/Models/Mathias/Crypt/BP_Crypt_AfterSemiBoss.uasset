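; BP_Crypt_AfterSemiBoss is an interactable crypt that becomes active once the semi-boss is beaten.
; Its point light starts dark, and the AfterSemiBossCryptAvailable event lights it and sets the BeatSemiBoss flag.
; Interact prints a debug string and, only when that flag is set, sends ABChangePositionMessage to the instigating character to change position.
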(event `self.ReceiveBeginPlay`
  ; Sets intensity for the crypt light
  (`LightComponent.SetIntensity` (`self.PointLight`) 0.0))

(event `/Game/Objects/BPI_CryptAvailable.AfterSemiBossCryptAvailable`
  ; "Turns" the crypt light on
  (`LightComponent.SetIntensity` (`self.PointLight`) 2000.0)
  (set `self.BeatSemiBoss` true))

(event `self.Interact`
  (params (CharacterInstigator :type "Character Object Reference"))
  ; Tells player to change position
  (`KismetSystemLibrary.PrintString` "You interacted")
  (if (`self.BeatSemiBoss`)
    (message `/Game/Input/BPI_ChangePos.ABChangePosition` CharacterInstigator)))

(fn `UserConstructionScript`)