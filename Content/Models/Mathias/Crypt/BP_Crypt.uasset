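; BP_Crypt is an interactable crypt actor that lights up when available and responds to a player holding the crypt key.
; Its point light starts dark on BeginPlay and switches on when the CryptAvailable event fires.
; InteractCPP prints a debug string, checks HoldsCryptKey on the first BP_PlayerCharacter found in the world, and if set calls ChangePositionMessage on the instigator.
; The Blueprint Interact event is empty.
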(event `/Game/Objects/BPI_CryptAvailable.CryptAvailable`
  ; "Turns" the crypt light on
  (`LightComponent.SetIntensity` (`self.PointLight`) 2000.0))

(event `self.ReceiveBeginPlay`
  ; Sets intensity for the crypt light
  (`LightComponent.SetIntensity` (`self.PointLight`) 0.0))

(event `/Game/Objects/BPI_Interact.Interact`
  (params (CharacterInstigator :type "Character Object Reference"))
  ; Tells player to change position
)

(event `self.InteractCPP`
  (params (CharacterInstigator :type "Character Object Reference"))
  ; Tells player to change position
  (bind _outactors (`GameplayStatics.GetAllActorsOfClass` "/Game/Characters/PlayerCharacter/BP_PlayerCharacter.BP_PlayerCharacter_C"))
  (`KismetSystemLibrary.PrintString` "You interacted")
  (if (`ToT_PlayerCharacter.HoldsCryptKey` (`|GetArrayItem` _outactors))
    (message `/Game/Input/BPI_ChangePos.ChangePosition` CharacterInstigator)))

(fn `UserConstructionScript`)