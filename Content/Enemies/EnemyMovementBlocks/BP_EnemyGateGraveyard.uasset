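; BP_EnemyGateGraveyard is an enemy block for the graveyard gate that spawns enemies while the player is inside its box.
; Box overlaps set PlayerInBox, which Tick checks through SpawnEnemies, with a Delay pacing spawns about two seconds apart.
; Each spawn randomly creates a zombie or bat AI offset from the player along world X.
; FindMovementBox replies to its instigator with InGateGraveyardMessage, identifying the block.
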(event `self.ReceiveBeginPlay`)

(event `self.ReceiveTick`
  (params (DeltaSeconds :type "Float (single-precision)"))
  (`self.SpawnEnemies`))

(event `self.FindMovementBox`
  (params (Instigator :type "Actor Object Reference"))
  (message `/Game/Enemies/EnemyMovementBlocks/BPI_MovementBlock.InGateGraveyard` Instigator))

(event `self.Box.OnComponentBeginOverlap`
  (params (OverlappedComponent :type "PrimitiveComponent Object Reference") (OtherActor :type "Actor Object Reference") (OtherComp :type "PrimitiveComponent Object Reference") (OtherBodyIndex :type Integer) (bFromSweep :type Boolean) (SweepResult :type "HitResult Structure (by ref)"))
  ; Knows Player has endered the block
  (if (`GameplayStatics.ObjectIsA` OtherActor "/Game/Characters/PlayerCharacter/BP_PlayerCharacter.BP_PlayerCharacter_C")
    (set `self.PlayerInBox` true)))

(event `self.Box.OnComponentEndOverlap`
  (params (OverlappedComponent :type "PrimitiveComponent Object Reference") (OtherActor :type "Actor Object Reference") (OtherComp :type "PrimitiveComponent Object Reference") (OtherBodyIndex :type Integer))
  ; Knows player has left this block
  (if (`GameplayStatics.ObjectIsA` OtherActor "/Game/Characters/PlayerCharacter/BP_PlayerCharacter.BP_PlayerCharacter_C")
    (set `self.PlayerInBox` false)))

(event `SpawnEnemies`
  ; Spawning enemies
  (if (`self.PlayerInBox`)
    (`KismetSystemLibrary.Delay` 2.0)
    (bind _output_get (set `self.EnemiesToSpawn` (`KismetMathLibrary.RandomInteger` 2)))
    (switch `int` _output_get
      (:`0`
        (`self.SpawnZombie`))
      (:`1`
        (`self.SpawnBat`)))))

(event `SpawnZombie`
  (bind (_returnvalue_x _returnvalue_y _returnvalue_z) (`KismetMathLibrary.BreakVector` (`self.K2_GetActorLocation` (`GameplayStatics.GetPlayerCharacter` 0))))
  ; Spawning enemies
  ;; Spawning zombie
  (`AIBlueprintHelperLibrary.SpawnAIFromClass` "/Game/Enemies/BP_Zombie.BP_Zombie_C" null (`KismetMathLibrary.MakeVector` (+ _returnvalue_x 500.0) _returnvalue_y (+ _returnvalue_z 50.0)) (struct) false null))

(event `SpawnBat`
  (bind (_returnvalue_x _returnvalue_y _returnvalue_z) (`KismetMathLibrary.BreakVector` (`self.K2_GetActorLocation` (`GameplayStatics.GetPlayerCharacter` 0))))
  ; Spawning enemies
  ;; Spawning bat
  (`AIBlueprintHelperLibrary.SpawnAIFromClass` "/Game/Enemies/BP_EnemyBat.BP_EnemyBat_C" null (`KismetMathLibrary.MakeVector` (+ _returnvalue_x 500.0) _returnvalue_y _returnvalue_z) (struct) false null))

(fn `UserConstructionScript`)