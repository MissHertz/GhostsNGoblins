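; BP_EnemyBat is a flying bat enemy with low health that damages the player on contact and is destroyed when health runs out.
; On spawn it derives a lane from its exact Y location and notifies overlapping movement blocks via BPI_FindMovementBlock.
; Area events for crypt and graveyard zones set hard-coded patrol bounds and Y position; the patrol movement itself is not here.
; Capsule hits check player distance, with a short cooldown between damage.
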(event `self.ReceiveBeginPlay`
  (`parent.ReceiveBeginPlay`)
  (bind _output_get (set `self.MaxHealth` 10.0))
  (set `self.CurrentHealth` _output_get)
  (`self.SetPositionMovementVariables`)
  (`self.SetBatPatrolPosition`)
  (`CharacterMovementComponent.SetMovementMode` (`self.CharacterMovement`) "MOVE_Flying" 0))

(event `self.AtCryptEnd`
  ; Setting movement variables
  ;; Setting patrol points
  (set `self.PatrolPointRight` 14030.0)
  (set `self.PatrolPointLeft` 12530.0)
  (set `self.MovementPosY` -2100.0))

(event `SetBatPatrolPosition`
  ; Setting movement variables
  ;; Finding out which box the bat is in
  (for _array_element (`PrimitiveComponent.GetOverlappingActors` (`self.CapsuleComponent`) "/Script/Engine.Actor")
    (if (`KismetSystemLibrary.DoesImplementInterface` _array_element "/Game/Enemies/EnemyMovementBlocks/BPI_FindMovementBlock.BPI_FindMovementBlock_C")
      (message `ToT_EnemyInMovementBlock.EnemyInMovementBlock` _array_element self))))

(event `self.CapsuleComponent.OnComponentHit`
  (params (HitComponent :type "PrimitiveComponent Object Reference") (OtherActor :type "Actor Object Reference") (OtherComp :type "PrimitiveComponent Object Reference") (NormalImpulse :type "Vector Structure") (Hit :type "HitResult Structure (by ref)"))
  (bind _returnvalue (`GameplayStatics.GetPlayerCharacter` 0))
  ; Melee Attack and damage
  ;; Bat colliding with player
  (if (<= (`self.GetDistanceTo` _returnvalue) 100.0)
    (if (not (`self.JustHit`))
      (`GameplayStatics.ApplyDamage` _returnvalue (`self.DamageToPlayer`))
      (set `self.JustHit` true)
      (`KismetSystemLibrary.Delay` 0.5)
      (set `self.JustHit` false))))

(event `self.AtCryptMiddle`
  ; Setting movement variables
  ;; Setting patrol points
  (set `self.PatrolPointRight` 10850.0)
  (set `self.PatrolPointLeft` 7830.0)
  (set `self.MovementPosY` -1830.0))

(event `self.AtCryptStart`
  ; Setting movement variables
  ;; Setting patrol points
  (set `self.PatrolPointRight` 7050.0)
  (set `self.PatrolPointLeft` 4725.0)
  (set `self.MovementPosY` -1700.0))

(event `self.ReceiveAnyDamage`
  (params (Damage :type "Float (single-precision)") (DamageType :type "DamageType Object Reference") (InstigatedBy :type "Controller Object Reference") (DamageCauser :type "Actor Object Reference"))
  ; Melee Attack and damage
  ;; Bat Taking Damage
  (if (> (`self.CurrentHealth`) 0.0)
    (set `self.CurrentHealth` (- (`self.CurrentHealth`) Damage))
    (if (<= (`self.CurrentHealth`) 0.0)
      (`KismetSystemLibrary.Delay` 0.1)
      (`self.K2_DestroyActor`))))

(event `self.AtUpperGraveyard`
  ; Setting movement variables
  ;; Setting patrol points
  (set `self.PatrolPointRight` 13600.0)
  (set `self.PatrolPointLeft` 8800.0)
  (set `self.MovementPosY` -230.0))

(event `SetPositionMovementVariables`
  ; Setting movement variables
  ;; Plan is for it to set where the enemy moves, if other plan does not work
  (`self.GetLane`)
  (switch `int` (`self.MovementLane`)
    (:`0`
      (set `self.LaneYPosition` 150.0))
    (:`1`
      (set `self.LaneYPosition` -100.0))
    (:`2`
      (set `self.LaneYPosition` 1700.0))
    (:`3`
      (set `self.LaneYPosition` 1450.0))))

(event `self.AtDownGraveyard`
  ; Setting movement variables
  ;; Setting patrol points
  (set `self.PatrolPointRight` 8090.0)
  (set `self.PatrolPointLeft` 3570.0)
  (set `self.MovementPosY` -500.0))

(event `self.AtCryptGraveyard`
  ; Setting movement variables
  ;; Setting patrol points
  (set `self.PatrolPointRight` 16050.0)
  (set `self.PatrolPointLeft` 14450.0)
  (set `self.MovementPosY` -300.0))

(event `GetLane`
  (bind (_returnvalue_x _returnvalue_y) (`KismetMathLibrary.BreakVector` (`self.K2_GetActorLocation`)))
  ; Setting movement variables
  ;; Finding lane enemy is in
  (if (== _returnvalue_y 150.0)
    (set `self.MovementLane` 0)
    (elif (== _returnvalue_y -100.0)
      (set `self.MovementLane` 1)
      (elif (== _returnvalue_y 1700.0)
        (set `self.MovementLane` 2)
        (else
          (set `self.MovementLane` 3))))))

(fn `UserConstructionScript`
  (`parent.UserConstructionScript`))