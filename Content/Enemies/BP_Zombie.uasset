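; Zombie enemy that starts chasing the player when the player is nearby in the same lane.
; A detection box overlap checks the player's distance and Y position against the zombie's lane, setting CanAttack and sending a chase event to its State Tree AI.
; A weighted random score-item drop (coin, necklace or money bag) is defined but currently disabled.
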(event `self.ReceiveBeginPlay`
  (`parent.ReceiveBeginPlay`))

(event `self.Box.OnComponentBeginOverlap`
  (params (OverlappedComponent :type "PrimitiveComponent Object Reference") (OtherActor :type "Actor Object Reference") (OtherComp :type "PrimitiveComponent Object Reference") (OtherBodyIndex :type Integer) (bFromSweep :type Boolean) (SweepResult :type "HitResult Structure (by ref)"))
  (bind _returnvalue (`GameplayStatics.GetPlayerCharacter` 0))
  (bind (_returnvalue_x _returnvalue_y) (`KismetMathLibrary.BreakVector` (`self.K2_GetActorLocation` _returnvalue)))
  ; Checks for player character when it is in range
  (if (<= (`self.GetDistanceTo` _returnvalue) 500.0)
    (if (== _returnvalue_y (`self.LaneYPosition`))
      (set `self.CanAttack` true)
      (`StateTreeComponent.SendStateTreeEvent` (`self.Zombie AI`) (`self.ChaseEvent`))
      (else
        (set `self.CanAttack` false :!label _label)))
    (else
      (goto _label))))

(event `self.PlayerOverlapBox.OnComponentBeginOverlap`
  (params (OverlappedComponent :type "PrimitiveComponent Object Reference") (OtherActor :type "Actor Object Reference") (OtherComp :type "PrimitiveComponent Object Reference") (OtherBodyIndex :type Integer) (bFromSweep :type Boolean) (SweepResult :type "HitResult Structure (by ref)")))

(event `DropScoreItem`
  ;[0.6979 0 0.02564 0.5] Dropping Score item, currently DISABLED
  (bind _output_get (set `self.ScoreItemDrop` (`KismetMathLibrary.RandomInteger` 10)))
  (switch `int` _output_get
    (:`0`
      (`KismetSystemLibrary.PrintString` "Dropping LOW score item" :!label _label_2)
      (`|SpawnActorFromClass` "/Game/Objects/ScoreItems/BP_ScoreItem_Coin.BP_ScoreItem_Coin_C" (`KismetMathLibrary.MakeTransform` (`self.K2_GetActorLocation`) (`self.K2_GetActorRotation`)) "Undefined" "MultiplyWithRoot" null null))
    (:`1`
      (goto _label_2))
    (:`2`
      (goto _label_2))
    (:`3`
      (`KismetSystemLibrary.PrintString` "Dropping MEDIUM score item" :!label _label_3)
      (`|SpawnActorFromClass` "/Game/Objects/ScoreItems/BP_ScoreItem_Necklace.BP_ScoreItem_Necklace_C" (`KismetMathLibrary.MakeTransform` (`self.K2_GetActorLocation`) (`self.K2_GetActorRotation`)) "Undefined" "MultiplyWithRoot" null null))
    (:`4`
      (goto _label_3))
    (:`5`
      (`KismetSystemLibrary.PrintString` "Dropping HIGH score item")
      (`|SpawnActorFromClass` "/Game/Objects/ScoreItems/BP_ScoreItem_MoneyBag.BP_ScoreItem_MoneyBag_C" (`KismetMathLibrary.MakeTransform` (`self.K2_GetActorLocation`) (`self.K2_GetActorRotation`)) "Undefined" "MultiplyWithRoot" null null))))

(fn `UserConstructionScript`
  (`parent.UserConstructionScript`))