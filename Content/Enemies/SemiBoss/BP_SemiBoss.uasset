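; Semi-boss enemy that sets its health and detection range on BeginPlay and takes damage from BP_Projectile overlaps on its capsule.
; Each hit applies damage to itself and subtracts the result from SemiBossHealthbar, while AnyDamage separately lowers CurrentHealth.
; Either value reaching zero flags death, but only the healthbar path sends the StateTree Dead event and notifies player characters.
; DestroyActor is never reached.
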(event `self.ReceiveBeginPlay`
  ; Setting up the semiboss
  (`parent.ReceiveBeginPlay`)
  (set `self.CurrentHealth` (`self.MaxHealth`))
  (bind _output_get (set `self.DetectionRange` 1900.0))
  (set `self.SemiBossDetectionRange` _output_get)
  (bind _output_get_2 (set `self.MaxHealth` 8.0))
  (set `self.CurrentHealth` _output_get_2))

(event `self.CapsuleComponent.OnComponentBeginOverlap`
  (params (OverlappedComponent :type "PrimitiveComponent Object Reference") (OtherActor :type "Actor Object Reference") (OtherComp :type "PrimitiveComponent Object Reference") (OtherBodyIndex :type Integer) (bFromSweep :type Boolean) (SweepResult :type "HitResult Structure (by ref)"))
  (if (`GameplayStatics.ObjectIsA` OtherActor "/Game/Weapons/BP_Projectile.BP_Projectile_C")
    (`KismetSystemLibrary.PrintString` "it's a projectile, will awpply damage now")
    (bind _returnvalue (`GameplayStatics.ApplyDamage` self 1.0))
    (`KismetSystemLibrary.PrintString` "damage was apparently applied")
    (bind _output_get (set `self.SemiBossHealthbar` (- (`self.SemiBossHealthbar`) _returnvalue)))
    (if (<= _output_get 0.0)
      (`KismetSystemLibrary.PrintString` "he's ded")
      (set `self.IsSemiBossDead` true)
      (`StateTreeComponent.SendStateTreeEvent` (`self.StateTree`) (`self.Dead`))
      (bind _outactors (`GameplayStatics.GetAllActorsOfClass` "/Game/Characters/PlayerCharacter/BP_PlayerCharacter.BP_PlayerCharacter_C"))
      (for _array_element _outactors
        (message `/Game/Objects/BPI_Key.HasBeatenSemiBoss` _array_element)))))

(event `self.ReceiveAnyDamage`
  (params (Damage :type "Float (single-precision)") (DamageType :type "DamageType Object Reference") (InstigatedBy :type "Controller Object Reference") (DamageCauser :type "Actor Object Reference"))
  (if (> (`self.CurrentHealth`) 0.0)
    (set `self.CurrentHealth` (- (`self.CurrentHealth`) Damage))
    (if (<= (`self.CurrentHealth`) 0.0)
      (set `self.IsSemiBossDead` true))))

(fn `UserConstructionScript`
  (`parent.UserConstructionScript`))