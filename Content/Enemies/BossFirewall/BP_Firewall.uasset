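; BP_Firewall is an enemy-area barrier that moves vertically when the player overlaps its trigger box, unless the matching boss is beaten.
; BeginPlay stores the starting Z and uses the "Boss" actor tag to mark it as a boss or semi-boss firewall.
; On overlap, it checks BeatBoss or BeatSemiBoss accordingly, then plays the FirewallMovement timeline, which offsets the actor's Z from its starting height.
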(event `self.ReceiveBeginPlay`
  (bind (_returnvalue_x _returnvalue_y _returnvalue_z) (`KismetMathLibrary.BreakVector` (`self.K2_GetActorLocation`)))
  (set `self.ActorZLocation` _returnvalue_z)
  (if (`self.ActorHasTag` self "Boss")
    (set `self.IsBossFirewall` true)
    (else
      (set `self.IsBossFirewall` false))))

(event `self.Box.OnComponentBeginOverlap`
  (params (OverlappedComponent :type "PrimitiveComponent Object Reference") (OtherActor :type "Actor Object Reference") (OtherComp :type "PrimitiveComponent Object Reference") (OtherBodyIndex :type Integer) (bFromSweep :type Boolean) (SweepResult :type "HitResult Structure (by ref)"))
  (bind (_returnvalue_x _returnvalue_y) (`KismetMathLibrary.BreakVector` (`self.K2_GetActorLocation`)))
  (if (`GameplayStatics.ObjectIsA` OtherActor "/Game/Characters/PlayerCharacter/BP_PlayerCharacter.BP_PlayerCharacter_C")
    (`KismetSystemLibrary.PrintString` "Player has overlapped")
    (if (`self.IsBossFirewall`)
      (if (not (`self.BeatBoss`))
        (bind (_direction _movement) (`Timeline|FirewallMovement` :!via `PlayFromStart` :!label _label)
          (:`Update`
            (`self.K2_SetActorLocation` (`KismetMathLibrary.MakeVector` _returnvalue_x _returnvalue_y (+ _movement (`self.ActorZLocation`)))))))
      (elif (not (`self.BeatSemiBoss`))
        (goto _label :!via `PlayFromStart`)))))

(fn `UserConstructionScript`)