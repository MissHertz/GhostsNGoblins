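; Enemy actor that attacks the player on entering its detection component and can be killed by damage.
; On overlap it snaps to face the player by comparing X positions, then after a short delay spawns a test weapon actor above itself, oriented from its yaw.
; Health starts at maximum, drops with any damage received, and the actor destroys itself when it reaches zero.
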(event `self.ReceiveBeginPlay`
  ; Setting the maximum health at the start
  (set `self.CurrentHealth` (`self.MaxHealth`)))

(event `self.Player detection.OnComponentBeginOverlap`
  (params (OverlappedComponent :type "PrimitiveComponent Object Reference") (OtherActor :type "Actor Object Reference") (OtherComp :type "PrimitiveComponent Object Reference") (OtherBodyIndex :type Integer) (bFromSweep :type Boolean) (SweepResult :type "HitResult Structure (by ref)"))
  (bind _returnvalue_x (`KismetMathLibrary.BreakVector` (`self.K2_GetActorLocation` OtherActor)))
  (bind _returnvalue_x_2 (`KismetMathLibrary.BreakVector` (`self.K2_GetActorLocation`)))
  ; Detects player
  (if (`GameplayStatics.ObjectIsA` OtherActor "/Game/Characters/PlayerCharacter/BP_PlayerCharacter.BP_PlayerCharacter_C")
    (if (< _returnvalue_x _returnvalue_x_2)
      (`self.K2_SetActorRotation` (struct :`Yaw` -180.0))
      (`self.AttackPlayer`)
      (`KismetSystemLibrary.PrintString` "Ay you in ma box!")
      (else
        (`self.K2_SetActorRotation` (struct))
        (`self.AttackPlayer`)
        (`KismetSystemLibrary.PrintString` "Ay you in ma box!")))))

(event `AttackPlayer`
  (bind (_returnvalue_x _returnvalue_y _returnvalue_z) (`KismetMathLibrary.BreakVector` (`self.K2_GetActorLocation`)))
  (bind (_returnvalue_roll _returnvalue_pitch _returnvalue_yaw) (`KismetMathLibrary.BreakRotator` (`self.K2_GetActorRotation`)))
  ; Attacks player
  (`KismetSystemLibrary.Delay` 0.2)
  (`|SpawnActorFromClass` "/Game/Weapons/BP_EnemyWeapon_TESTER.BP_EnemyWeapon_TESTER_C" (`KismetMathLibrary.MakeTransform` (`KismetMathLibrary.MakeVector` _returnvalue_x _returnvalue_y (+ _returnvalue_z 100.0)) (`KismetMathLibrary.MakeRotator` 0.0 0.0 (* _returnvalue_yaw -1.0))) "AdjustIfPossibleButAlwaysSpawn" "MultiplyWithRoot" null null))

(event `self.ReceiveAnyDamage`
  (params (Damage :type "Float (single-precision)") (DamageType :type "DamageType Object Reference") (InstigatedBy :type "Controller Object Reference") (DamageCauser :type "Actor Object Reference"))
  ; Enemy gettong hit/killed
  (if (> (`self.CurrentHealth`) 0.0)
    (bind _output_get (set `self.CurrentHealth` (- (`self.CurrentHealth`) Damage)))
    (`KismetSystemLibrary.PrintString` (`KismetStringLibrary.Conv_DoubleToString` _output_get))
    (if (<= (`self.CurrentHealth`) 0.0)
      (`self.K2_DestroyActor`))))

(fn `UserConstructionScript`)