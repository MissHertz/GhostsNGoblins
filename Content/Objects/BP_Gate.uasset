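; Interactable gate that swings open when the player holds the crypt key.
; InteractCPP checks HoldsCryptKey on the first ToT_PlayerCharacter found, then looks up BP_Gate actors in the level tagged Left and Right.
; Each side's loop starts its own timeline (LeftGateOpen or RightGateOpen), whose track drives the gate's yaw through SetActorRotation.
; The plain Interact event is empty.
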(event `/Game/Objects/BPI_Interact.Interact`
  (params (CharacterInstigator :type "Character Object Reference"))
  ; Gate "Opening" animation
)

(event `self.InteractCPP`
  (params (CharacterInstigator :type "Character Object Reference"))
  ; Gate "Opening" animation
  (bind _outactors (`GameplayStatics.GetAllActorsOfClass` "/Script/GhostsNGoblins_BP.ToT_PlayerCharacter"))
  (if (`ToT_PlayerCharacter.HoldsCryptKey` (`|GetArrayItem` _outactors))
    (`|ExecutionSequence`
      (:`then_0`
        (bind _outactors_2 (`GameplayStatics.GetAllActorsOfClassWithTag` "BP_Gate_C" "Left"))
        (for _array_element _outactors_2
          (bind (_direction _newtrack_0) (`Timeline|LeftGateOpen` :!via `PlayFromStart`)
            (:`Update`
              (`self.K2_SetActorRotation` _array_element (`KismetMathLibrary.MakeRotator` 0.0 0.0 _newtrack_0) false)))))
      (:`then_1`
        (bind _outactors_3 (`GameplayStatics.GetAllActorsOfClassWithTag` "BP_Gate_C" "Right"))
        (for _array_element_2 _outactors_3
          (bind (_direction_2 _newtrack_0_2) (`Timeline|RightGateOpen` :!via `PlayFromStart`)
            (:`Update`
              (`self.K2_SetActorRotation` _array_element_2 (`KismetMathLibrary.MakeRotator` 0.0 0.0 _newtrack_0_2) false))))))))

(fn `UserConstructionScript`)