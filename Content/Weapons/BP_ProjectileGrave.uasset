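; BP_ProjectileGrave is a projectile base actor that damages the player character on overlap.
; On BeginPlay it runs SetDamage and SetTimeExsistance, overridable events that let child classes define damage and lifetime, then destroys itself once that lifetime elapses.
; A capsule overlap applies the damage only to BP_PlayerCharacter and leaves the projectile alive until its timer ends.
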(event `self.ReceiveBeginPlay`
  ; Lifespan
  (`self.SetDamage`)
  (`self.SetTimeExsistance`)
  (`KismetSystemLibrary.Delay` (`self.ProjectileTime`))
  (`self.K2_DestroyActor`))

(event `self.Capsule.OnComponentBeginOverlap`
  (params (OverlappedComponent :type "PrimitiveComponent Object Reference") (OtherActor :type "Actor Object Reference") (OtherComp :type "PrimitiveComponent Object Reference") (OtherBodyIndex :type Integer) (bFromSweep :type Boolean) (SweepResult :type "HitResult Structure (by ref)"))
  (if (`GameplayStatics.ObjectIsA` OtherActor "/Game/Characters/PlayerCharacter/BP_PlayerCharacter.BP_PlayerCharacter_C")
    (`GameplayStatics.ApplyDamage` OtherActor (`self.Damage`))))

(event `SetDamage`
  ; Allowing to set damage for all children
  (set `self.Damage` 1.0))

(event `SetTimeExsistance`
  ; Allowing to set time of exsistance for all children
  (set `self.ProjectileTime` 6.0))

(fn `UserConstructionScript`)