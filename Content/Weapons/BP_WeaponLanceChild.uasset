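; Lance weapon Blueprint, a child of a parent weapon class, that attacks by firing a lance projectile.
; Attack spawns BP_ProjectileLance_Child at the world transform of the weapon mesh's WeaponSocket.
; SendMessage finds all BP_PlayerCharacter actors and calls HoldsLanceMessage on them.
; BeginPlay runs the parent logic and prints a debug string.
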(event `self.ReceiveBeginPlay`
  (`parent.ReceiveBeginPlay`)
  (`KismetSystemLibrary.PrintString` "It has gone through"))

(event `self.Send message`
  (bind _outactors (`GameplayStatics.GetAllActorsOfClass` "/Game/Characters/PlayerCharacter/BP_PlayerCharacter.BP_PlayerCharacter_C"))
  (message `/Game/Weapons/BPI_Weapon.HoldsLance` _outactors))

(event `/Game/Input/BPI_Interact.Attack`
  (`|SpawnActorFromClass` "/Game/Weapons/BP_ProjectileLance_Child.BP_ProjectileLance_Child_C" (`SceneComponent.GetSocketTransform` (`self.WeaponMesh`) "WeaponSocket" "RTS_World") "Undefined" "MultiplyWithRoot" null null))

(fn `UserConstructionScript`
  (`parent.UserConstructionScript`))